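; Networked gun actor, parented to a player character, that handles firing, ammo and reloading.
; The authority counts down fire rate and rounds; BeginPlay and Fire push ammo to the owner's HUD, locally or via client event.
; Fire traces a predicted projectile path, plays sound and arms montage, then server-side damages the hit HealthComponent and credits kills.
; A helper computes accuracy spread by blending random and aim directions, though Fire itself never calls it.
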(event EventBeginPlay
  (bind _returnvalue (Actor|GetParentActor))
  (bind _magazinesize (Variables|Default|GetMagazineSize))
  (Variables|Default|SetRoundsRemainingInMagazine (Variables|Default|GetMagazineSize))
  (Utilities|IsValid _returnvalue :!label _label
    (:Is%20Valid
      (bind _asplayer_character_blueprint (Utilities|Casting|CastToPlayerCharacterBlueprint _returnvalue))
      (if (Pawn|IsLocallyControlled _asplayer_character_blueprint)
        (Default|UpdateAmmoHUDEvent _asplayer_character_blueprint (Variables|Default|GetRoundsRemainingInMagazine) _magazinesize)
        (else
          (Default|ClientUpdateAmmoHUDEvent _asplayer_character_blueprint (Variables|Default|GetRoundsRemainingInMagazine) _magazinesize))))
    (:Is%20Not%20Valid
      (Utilities|FlowControl|Delay 0.1)
      (goto _label))))

(event Collision|EventActorBeginOverlap
  (params (OtherActor :type Actor%20Object%20Reference)))

(event EventTick
  (params (DeltaSeconds :type Float%20%28single-precision%29))
  (Networking|SwitchHasAuthority
    (:Authority
      (if (not (Variables|Default|GetbCanFire))
        (bind _output_get (Variables|Default|SetTimeTillNextShot (- (Variables|Default|GetTimeTillNextShot) DeltaSeconds)))
        (if (and (<= _output_get 0.0) (> (Variables|Default|GetRoundsRemainingInMagazine) 0))
          (Variables|Default|SetbCanFire true))))))

(fn ConstructionScript)

(fn Fire
  (params (LaunchDirection :type Vector))
  (bind _returnvalue (Actor|GetParentActor))
  (bind _muzzleposition (Variables|Default|GetMuzzlePosition))
  (bind _magazinesize (Variables|Default|GetMagazineSize))
  (bind _returnvalue_2 (Transformation|GetWorldLocation _muzzleposition))
  (if (Variables|Default|GetbCanFire)
    (Networking|SwitchHasAuthority
      (:Authority
        (Variables|Default|SetbCanFire false)
        (Variables|Default|SetTimeTillNextShot (Variables|Default|GetFireRate))
        (bind _output_get (Variables|Default|SetRoundsRemainingInMagazine (- (Variables|Default|GetRoundsRemainingInMagazine) 1)))
        (bind _asplayer_character_blueprint (Utilities|Casting|CastToPlayerCharacterBlueprint (Actor|GetParentActor))
          (:then
            (if (Pawn|IsLocallyControlled _asplayer_character_blueprint)
              (Default|UpdateAmmoHUDEvent _asplayer_character_blueprint _output_get _magazinesize)
              (else
                (Default|ClientUpdateAmmoHUDEvent _asplayer_character_blueprint _output_get _magazinesize))))
          (:CastFailed
            _)))
      (:Remote
        _))
    (bind _outhit (Class|GameplayStatics|BlueprintPredictProjectilePathbyTraceChannel _returnvalue_2 (* LaunchDirection (Variables|Default|GetMuzzleVelocity)) true 1.0 "ECC_WorldDynamic" false 0 "None"))
    (Audio|PlaySoundatLocation "/Game/Assets/Audio/FirstPersonTemplateWeaponFire02.FirstPersonTemplateWeaponFire02" _returnvalue_2 "0, 0, 0" 1.0 1.0 0.0 0 0 0)
    (bind _asplayer_character_blueprint_2 (Utilities|Casting|CastToPlayerCharacterBlueprint (Actor|GetParentActor)))
    (Animation|Montage|MontagePlay (Components|SkeletalMesh|GetAnimInstance (Variables|/Game/Blueprints/PlayerCharacterBlueprint.PlayerCharacterBlueprint_C|GetArms _asplayer_character_blueprint_2)) "/Game/Assets/Animations/FirstPersonFire_Montage.FirstPersonFire_Montage" 1.0 "MontageLength" 0.0 true)
    (Utilities|IsValid (.HitActor (Collision|BreakHitResult _outhit))
      (:Is%20Valid
        (if (and (Networking|IsServer) (Utilities|IsValid (Actor|GetComponentbyClass (.HitActor (Collision|BreakHitResult _outhit)) "/Script/AGPAssessmnt4Group17.HealthComponent")))
          (bind _returnvalue_3 (Class|HealthComponent|OnTakeDamage (Actor|GetComponentbyClass (.HitActor (Collision|BreakHitResult _outhit)) "/Script/AGPAssessmnt4Group17.HealthComponent") (Variables|Default|GetBulletDamage)))
          (if (<= _returnvalue_3 0.0)
            (Utilities|IsValid _returnvalue
              (:Is%20Valid
                (bind _asplayer_character_blueprint_3 (Utilities|Casting|CastToPlayerCharacterBlueprint _returnvalue))
                (if (Utilities|IsValid _asplayer_character_blueprint_3)
                  (Class|PlayerCharacter|UpdateKillCount _asplayer_character_blueprint_3))))))))))

(fn Reload
  (Variables|Default|SetRoundsRemainingInMagazine (Variables|Default|GetMagazineSize)))

(fn CalculateAccuracyOffsetVector
  (params (FireDirection :type Vector))
  (return (Math|Vector|Lerp(Vector) (Math|Random|RandomUnitVector) (Math|Vector|Normalize FireDirection) (Math|Float|Sqrt (Variables|Default|GetWeaponAccuracy)))))